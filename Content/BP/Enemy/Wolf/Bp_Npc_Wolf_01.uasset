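; Wolf enemy NPC Blueprint that tracks whether the character is alive and carries a health bar widget.
; On death it clears the alive flag, zeroes walk speed and sets a short lifespan so the actor is removed shortly afterward.
; Every Tick it rotates the health bar toward the player camera, billboard-style.
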(event `self.ReceiveBeginPlay`
  (set `self.Is Alive?` true))

(event `self.OnCharacterDead`
  (set `self.Is Alive?` false)
  (set `CharacterMovementComponent.MaxWalkSpeed` 0.0 (`self.CharacterMovement`))
  (`self.SetLifeSpan` 2.0))

(event `self.ReceiveTick`
  (params (DeltaSeconds :type "Float (single-precision)"))
  (bind _healthbarwidget (`self.HealthBarWidget`))
  (`SceneComponent.K2_SetWorldRotation` _healthbarwidget (`KismetMathLibrary.FindLookAtRotation` (`SceneComponent.K2_GetComponentLocation` _healthbarwidget) (`PlayerCameraManager.GetCameraLocation` (`GameplayStatics.GetPlayerCameraManager` 0))) false false))

(fn `UserConstructionScript`)