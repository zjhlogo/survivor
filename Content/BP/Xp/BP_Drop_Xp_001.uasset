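; XP drop actor that drives a Niagara particle system and feeds it the player's location.
; On BeginPlay it registers itself as the particle data callback and sets a looping timer that calls Cus_Spawn to activate the system.
; For each exported particle it updates the ActorLocation variable from the player character and tests proximity to the particle.
; The proximity branch is empty, so no XP is awarded here.
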(event `self.ReceiveBeginPlay`
  (`KismetSystemLibrary.K2_SetTimer` null "Cus_Spawn" 0.0 true)
  (`NiagaraComponent.SetNiagaraVariableObject` (`self.Niagara`) "BPCalback" self))

(event `Cus_Spawn`
  (`ActorComponent.SetActive` (`self.Niagara`) true false))

(event `self.ReceiveParticleData`
  (params (Data :type "Array of BasicParticleData Structure (by ref)") (NiagaraSystem :type "NiagaraSystem Object Reference") (SimulationPositionOffset :type "Vector Structure (by ref)"))
  (bind _returnvalue (`SceneComponent.K2_GetComponentLocation` (`Actor.RootComponent` (`GameplayStatics.GetPlayerCharacter` 0))))
  (for _array_element Data
    (`NiagaraComponent.SetVariableVec3` (`self.Niagara`) "ActorLocation" _returnvalue)
    (if (< (`KismetMathLibrary.Vector_Distance` _returnvalue (break `BasicParticleData` _array_element)) 100.0)
      _)))

(fn `UserConstructionScript`)