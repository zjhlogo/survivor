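; BP_Laser is a laser beam actor that stretches a beam effect along its forward vector up to a maximum length.
; Each tick, a thin sphere trace on the Projectile profile finds the first hit and sets the particle beam's target to the impact point, or to full length on a miss.
; While hitting, it also spawns an auto-release pooled impact effect every tick; it applies no damage here.
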(event `self.ReceiveTick`
  (params (DeltaSeconds :type "Float (single-precision)"))
  (bind _returnvalue (`self.K2_GetActorLocation`))
  (bind _p_fx_beam_jiguang (`self.P_Fx_Beam_jiguang`))
  (bind _returnvalue_2 (+ _returnvalue (* (`self.GetActorForwardVector`) (`self.GetLaserBeamMaxLength`))))
  (bind (_outhit _returnvalue_3) (`KismetSystemLibrary.SphereTraceSingleByProfile` _returnvalue _returnvalue_2 0.1 "Projectile"))
  (if _returnvalue_3
    (`ParticleSystemComponent.SetBeamTargetPoint` _p_fx_beam_jiguang 0 (`.ImpactPoint` (`GameplayStatics.BreakHitResult` _outhit)) 0)
    (`NiagaraFunctionLibrary.SpawnSystemAtLocation` "/Game/Art/Effect/Niagara/BlueLaser/Fx_Ng_Hit_impact.Fx_Ng_Hit_impact" (`.ImpactPoint` (`GameplayStatics.BreakHitResult` _outhit)) (`self.K2_GetActorRotation`) (1.0 1.0 1.0) true true "AutoRelease") ; 过程中
    (else
      (`ParticleSystemComponent.SetBeamTargetPoint` _p_fx_beam_jiguang 0 _returnvalue_2 0))))

(fn `UserConstructionScript`)