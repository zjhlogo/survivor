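; Generated dynamic mesh actor that builds a solid heightmap mesh from a texture, with complex-as-simple collision.
; On rebuild it tessellates a grid, displaces it by the texture, extrudes it by Height, then smooths and recomputes normals.
; Depending on the edge-clip flag, a plane cut first removes invalid height values and re-bases the mesh before extrusion.
; The construction script applies the material, and ConvertToStaticMesh saves the result as a Nanite static mesh asset.
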(event `self.OnRebuildGeneratedMesh`
  (params (TargetMesh :type "DynamicMesh Object Reference"))
  (bind `_尺寸大小` (`self.尺寸大小`))
  (set `self.Dynamic Mesh` TargetMesh)
  (`|ExecutionSequence`
    (:`then_0`
      (bind _returnvalue (`GeometryScriptLibrary_MeshPrimitiveFunctions.AppendRectangleXY` (`self.Dynamic Mesh`) (struct) (struct) `_尺寸大小` `_尺寸大小` 10 10 null))
      (bind _returnvalue_2 (`GeometryScriptLibrary_MeshSubdivideFunctions.ApplyPNTessellation` _returnvalue (struct) (`self.曲面细分级别`) null))
      (`GeometryScriptLibrary_MeshDeformFunctions.ApplyDisplaceFromTextureMap` _returnvalue_2 (`self.Texture`) (struct) (make `GeometryScriptDisplaceFromTextureOptions` (`self.图片拉伸`)) 0 null)
      (if (`self.边缘裁剪`)
        (`GeometryScriptLibrary_MeshModelingFunctions.ApplyMeshLinearExtrudeFaces` (`self.Dynamic Mesh`) (make `GeometryScriptMeshLinearExtrudeOptions` (`self.Height`)) (struct) null)
        (else
          ;[1 1 1] 去除边界无效值再进行拉伸
          (bind _returnvalue_3 (`GeometryScriptLibrary_MeshBooleanFunctions.ApplyMeshPlaneCut` (`self.Dynamic Mesh`) (`KismetMathLibrary.MakeTransform` (`KismetMathLibrary.MakeVector` 0.0 0.0 (`self.无效值域`))) (make `GeometryScriptMeshPlaneCutOptions` false false true) null))
          (bind _returnvalue_4 (`GeometryScriptLibrary_MeshTransformFunctions.TransformMesh` _returnvalue_3 (`KismetMathLibrary.MakeTransform` (`KismetMathLibrary.MakeVector` 0.0 0.0 (* (`self.无效值域`) -1.0))) true null))
          (`GeometryScriptLibrary_MeshModelingFunctions.ApplyMeshLinearExtrudeFaces` (`self.Dynamic Mesh`) (make `GeometryScriptMeshLinearExtrudeOptions` (`self.Height`) "FixedDirection" (0.0 0.0 1.0) "EntireSelection" (struct :`GroupMode` "PreserveExisting") 1.0 false) (struct) null)))
      (bind _returnvalue_5 (`GeometryScriptLibrary_MeshDeformFunctions.ApplyIterativeSmoothingToMesh` (`self.Dynamic Mesh`) (struct) (make `GeometryScriptIterativeMeshSmoothingOptions` (`self.模型细分`)) null))
      (`GeometryScriptLibrary_MeshNormalsFunctions.RecomputeNormals` _returnvalue_5 (make `GeometryScriptCalculateNormalsOptions` false false) null)
      (`PrimitiveComponent.SetCollisionEnabled` (`self.DynamicMeshComponent`) "QueryAndPhysics")
      (`DynamicMeshComponent.EnableComplexAsSimpleCollision` (`self.DynamicMeshComponent`)))))

(fn `Convert to Static Mesh`
  (bind _returnvalue (`BaseDynamicMeshComponent.GetDynamicMesh` (`self.DynamicMeshComponent`)))
  (`GeometryScriptLibrary_CreateNewAssetFunctions.CreateNewStaticMeshAssetFromMesh` _returnvalue (`KismetStringLibrary.Concat_StrStr` (`self.Asset Path`) (`self.Name`)) (make `GeometryScriptCreateNewStaticMeshAssetOptions` false false true) null
    (:`Failure`
      (`KismetSystemLibrary.PrintText` "没有创建成功"))
    (:`Success`
      (`KismetSystemLibrary.PrintText` "创建成功"))))

(fn `UserConstructionScript`
  (`PrimitiveComponent.SetMaterial` (`self.DynamicMeshComponent`) 0 (`self.Material`)))