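; Wolf NPC monster Blueprint that handles its death and keeps its health bar facing the player's camera.
; On death it clears its alive flag, stops and disables character movement, and sets a short lifespan so the actor is removed shortly after.
; Every Tick rotates the health bar widget toward the first player's camera with a look-at rotation, acting as a manual billboard.
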(event `self.OnDead`
  (bind _charactermovement (`self.CharacterMovement`))
  (set `self.Is Alive?` false)
  (set `CharacterMovementComponent.MaxWalkSpeed` 0.0 _charactermovement)
  (`CharacterMovementComponent.DisableMovement` _charactermovement)
  (`self.SetLifeSpan` 2.5))

(event `self.ReceiveTick`
  (params (DeltaSeconds :type "Float (single-precision)"))
  (bind _healthbarwidget (`self.HealthBarWidget`))
  (`SceneComponent.K2_SetWorldRotation` _healthbarwidget (`KismetMathLibrary.FindLookAtRotation` (`SceneComponent.K2_GetComponentLocation` _healthbarwidget) (`PlayerCameraManager.GetCameraLocation` (`GameplayStatics.GetPlayerCameraManager` 0))) false false))

(fn `UserConstructionScript`)