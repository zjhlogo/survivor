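; AI controller for the BombBug monster that starts its behavior tree on possession and feeds it sight information.
; Perception updates set the LookPlayer blackboard flag on successful sight and clear it for any other stimulus.
; On a successful sighting it also sets a close-range flag from the bug's distance to player pawn 0, whichever actor was sensed.
; That range flag refreshes only on those sighting events.
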(event `self.ReceivePossess`
  (params (PossessedPawn :type "Pawn Object Reference"))
  (bind _asbp_npc_bomb_bug (cast `/Game/BP/Monster/003_BombBug/Bp_Npc_BombBug` PossessedPawn))
  (set `self.As Bp Npc Bomb Bug` _asbp_npc_bomb_bug)
  (`self.RunBehaviorTree` "/Game/BP/Monster/003_BombBug/BT_Npc_BombBug.BT_Npc_BombBug"))

(event `self.AIPerception.OnTargetPerceptionUpdated`
  (params (Actor :type "Actor Object Reference") (Stimulus :type "AIStimulus Structure"))
  (bind _returnvalue (`AIBlueprintHelperLibrary.GetBlackboard` null))
  (bind _returnvalue_2 (`AIBlueprintHelperLibrary.GetBlackboard` null))
  (set `self.Actor` Actor)
  (bind _returnvalue_3 (`AIPerceptionSystem.GetSenseClassForStimulus` Stimulus))
  (if (and (== _returnvalue_3 "/Script/AIModule.AISense_Sight") (`.bSuccessfullySensed` (break `AIStimulus` Stimulus)))
    (`BlackboardComponent.SetValueAsBool` _returnvalue_2 "LookPlayer" true)
    (if (<= (`KismetMathLibrary.Vector_Distance` (`self.K2_GetActorLocation` (`self.As Bp Npc Bomb Bug`)) (`self.K2_GetActorLocation` (`GameplayStatics.GetPlayerPawn` 0))) 500.0)
      (`BlackboardComponent.SetValueAsBool` _returnvalue "DistanceToTarget<500 " true)
      (else
        (`BlackboardComponent.SetValueAsBool` _returnvalue "DistanceToTarget<500 " false)))
    (else
      (`BlackboardComponent.SetValueAsBool` _returnvalue_2 "LookPlayer" false))))

(fn `UserConstructionScript`)