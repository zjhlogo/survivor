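; Bomb bug monster NPC with separate ground and air attacks and a camera-facing health bar.
; Tick runs a delay-based macro that randomly toggles IsAir, which gates Attack on the ground and Attack02 in the air.
; Both attacks set flags, then run timelines driving emissive glow through dynamic material instances recreated each update.
; Ground attacks halt walking until ResetMovement restores it; death disables movement and destroys the actor shortly after.
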(event `self.OnDead`
  (bind _charactermovement (`self.CharacterMovement`))
  ;[1 1 1] 注释
  (set `self.Is Alive?` false)
  (set `CharacterMovementComponent.MaxWalkSpeed` 0.0 _charactermovement)
  (`CharacterMovementComponent.DisableMovement` _charactermovement)
  (`self.SetLifeSpan` 2.0))

(event `Attack`
  ;[1 1 1] 注释
  (if (`self.Is Alive?`)
    (if (not (`self.IsAir?`))
      (`|ExecutionSequence`
        (:`then_0`
          (set `CharacterMovementComponent.MaxWalkSpeed` 0.0 (`self.CharacterMovement`))
          (set `self.Attack?` true)
          (`KismetSystemLibrary.Delay` 1.5)
          (bind (_direction _0_1) (`Timeline|时间轴` :!via `PlayFromStart`)
            (:`Update`
              (`self.SetMaterial` _0_1)
              (`KismetSystemLibrary.Delay` (`self.AttackAnimationTime`)))))))))

(event `ResetMovement`
  ;[1 1 1] 注释
  (set `self.Attack?` false)
  (set `CharacterMovementComponent.MaxWalkSpeed` 200.0 (`self.CharacterMovement`)))

(event `Attack02`
  ;[1 1 1] 注释
  (if (`self.Is Alive?`)
    (if (`self.IsAir?`)
      (`|ExecutionSequence`
        (:`then_0`
          (set `self.Attack02?` true)
          (`KismetSystemLibrary.Delay` 1.5)
          (bind (_direction _0_1) (`Timeline|时间轴_0` :!via `PlayFromStart`)
            (:`Update`
              (`self.SetMaterial` _0_1)
              (`KismetSystemLibrary.Delay` (`self.AttackAnimationTime`))
              (set `self.Attack02?` (`KismetMathLibrary.RandomBool`)))))))))

(event `self.ReceiveTick`
  (params (DeltaSeconds :type "Float (single-precision)"))
  (bind _healthbarwidget (`self.HealthBarWidget`))
  ;[1 1 1] 注释
  (`SceneComponent.K2_SetWorldRotation` _healthbarwidget (`KismetMathLibrary.FindLookAtRotation` (`SceneComponent.K2_GetComponentLocation` _healthbarwidget) (`PlayerCameraManager.GetCameraLocation` (`GameplayStatics.GetPlayerCameraManager` 0))) false false)
  (`|ExecutionSequence`
    (:`then_0`
      (`self.Set IsAir`))))

(fn `SetMaterial`
  (params (Value :type "Float (double-precision)"))
  (bind _returnvalue (`PrimitiveComponent.CreateDynamicMaterialInstance` (`self.Mesh`) 0 "/Game/Art_Test/NPC/BombBug/Materials/MI_Npc_Bombbug.MI_Npc_Bombbug" "None"))
  (`MaterialInstanceDynamic.SetScalarParameterValue` _returnvalue "EmissColor" Value))

(fn `UserConstructionScript`)